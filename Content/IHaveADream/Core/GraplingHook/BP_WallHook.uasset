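; BP_WallHook is the grappling hook projectile that lets its instigating player grapple to walls.
; On BeginPlay it tells InstigatorPlayer to start the grapple, passing itself as the hook.
; When its collision component hits an actor tagged "WallHook", it triggers the player's pull to the wall and stops its projectile movement.
; Any other hit tells the player to stop the grapple.
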(event `self.ReceiveBeginPlay`
  (`/Game/IHaveADream/Player/BP_FirstPersonCharacter.StartGrappleToWall` (`self.InstigatorPlayer`) self))

(event `self.CollisionComponent.OnComponentHit`
  (params (HitComponent :type "PrimitiveComponent Object Reference") (OtherActor :type "Actor Object Reference") (OtherComp :type "PrimitiveComponent Object Reference") (NormalImpulse :type "Vector Structure") (Hit :type "HitResult Structure (by ref)"))
  (if (`self.ActorHasTag` OtherActor "WallHook")
    (`/Game/IHaveADream/Player/BP_FirstPersonCharacter.StartGrapplePullToWall` (`self.InstigatorPlayer`))
    (`MovementComponent.StopMovementImmediately` (`self.ProjectileMovement`))
    (else
      (`/Game/IHaveADream/Player/BP_FirstPersonCharacter.StopGrappleToWall` (`self.InstigatorPlayer`)))))

(fn `UserConstructionScript`
  (`parent.UserConstructionScript`))