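; A dialogue trigger actor that shows a dialogue widget and plays a sound when a Player-tagged actor overlaps its box.
; The widget stays on screen for the sound's duration, then is removed.
; CzasTrwania holds that duration during playback, and CzyDalejTrwa compares it against delta time as a retrigger guard.
; Despite its name ("is it still going"), that function returns true when no playback remains, so the dialogue can replay afterwards.
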(event `self.Box.OnComponentBeginOverlap`
  (params (OverlappedComponent :type "PrimitiveComponent Object Reference") (OtherActor :type "Actor Object Reference") (OtherComp :type "PrimitiveComponent Object Reference") (OtherBodyIndex :type Integer) (bFromSweep :type Boolean) (SweepResult :type "HitResult Structure (by ref)"))
  (bind _sound (`self.Sound`))
  (bind _duration (`SoundBase.Duration` _sound))
  (if (`self.ActorHasTag` OtherActor "Player")
    (bind _skonczylo_sie (`self.Czy dalej trwa?` (`self.czas trwania`)))
    (if _skonczylo_sie
      (bind _returnvalue (`|CreateWidget` "/Game/IHaveADream/Menu/UI/DialogWidget.DialogWidget_C"))
      (`UserWidget.AddToViewport` _returnvalue 0)
      (`GameplayStatics.PlaySoundAtLocation` _sound (`self.K2_GetActorLocation`) (struct) 1.0 1.0 0.0 null null null null)
      (set `self.czas trwania` _duration)
      (`KismetSystemLibrary.Delay` _duration)
      (`Widget.RemoveFromParent` _returnvalue)
      (set `self.czas trwania` 0.0))))

(fn `Czy dalej trwa?`
  (params (`duration of sound` :type "Float (double-precision)"))
  (returns (`skonczylo sie` :type Boolean))
  (set `self.Clock` `duration of sound`)
  (bind _output_get (set `self.skonczylo sie` (<= (- (`self.Clock`) (`GameplayStatics.GetWorldDeltaSeconds`)) 0.0)))
  (return _output_get))

(fn `UserConstructionScript`)